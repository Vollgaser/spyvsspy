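; Gameplay character with an adjustable spring-arm camera, walking and jumping.
; Input events from the PlayerControllerInputs graph drive clamped camera rotation, arm-length zoom, movement and Jump; both click actions are empty.
; Forward movement follows player controller 0's yaw, while strafing follows the actor's rotation.
; BeginPlay applies default distance, speed and FOV; WhoPossessesActor reports player or AI control, and an FOV-zoom branch sits unconnected.
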(event EventBeginPlay
  (CallFunction|SetDefaultValues))

(fn ConstructionScript)

(fn RotateCamera
  (params (RotationValue :type Vector%202D%20Structure))
  (bind _springarm (Variables|Default|GetSpringArm))
  (bind _valuerangeofcamerapitch (Variables|DesignerVariables|GetValueRangeOfCameraPitch))
  (bind _camerasensitivity (Variables|DesignerVariables|GetCameraSensitivity))
  (bind _valuerangeofcamerayaw (Variables|DesignerVariables|GetValueRangeOfCameraYaw))
  (bind _returnvalue (* RotationValue _camerasensitivity))
  (bind _relativerotation (Variables|/Script/Engine.SceneComponent|GetRelativeRotation _springarm))
  (bind (_x _y) (Math|Vector2D|BreakVector2D _returnvalue))
  (Transformation|SetRelativeRotation (Variables|Default|GetSpringArm) (Math|Rotator|MakeRotator 0.0 (Math|Float|Clamp(Float) (+ (.pitch _relativerotation) _y) (.x _valuerangeofcamerapitch) (.y _valuerangeofcamerapitch)) (Math|Float|Clamp(Float) (+ (.yaw _relativerotation) _x) (.x _valuerangeofcamerayaw) (.y _valuerangeofcamerayaw))) false false))

(fn CameraZoom
  (params (ZoomValue :type Float%20%28double-precision%29))
  (bind _valuerangecameradistance (Variables|DesignerVariables|CameraZoom|GetValueRangeCameraDistance))
  (bind _springarm (Variables|Default|GetSpringArm))
  (Variables|/Script/Engine.SpringArmComponent|SetTargetArmLength _springarm (Math|Float|Clamp(Float) (+ (Variables|/Script/Engine.SpringArmComponent|GetTargetArmLength _springarm) (* ZoomValue (Variables|Default|Getzoom%20change%20in%20UU%20per%20steps%20))) (.x _valuerangecameradistance) (.y _valuerangecameradistance))))

(fn Moving
  (params (MovementValue :type Vector%202D%20Structure))
  (bind _returnvalue (Transformation|GetActorRotation))
  (bind (_x _y) (Math|Vector2D|BreakVector2D MovementValue))
  (Pawn|Input|AddMovementInput (Math|Vector|GetRightVector (Math|Rotator|MakeRotator (.roll _returnvalue) 0.0 (.yaw _returnvalue))) _x false)
  (Pawn|Input|AddMovementInput (Math|Vector|GetForwardVector (Math|Rotator|MakeRotator 0.0 0.0 (.yaw (Transformation|GetActorRotation (Game|GetPlayerController 0))))) _y false))

(fn SetDefaultValues
  (Variables|/Script/Engine.SpringArmComponent|SetTargetArmLength (Variables|Default|GetSpringArm) (Variables|DesignerVariables|GetCameraDistance))
  (Variables|/Script/Engine.CharacterMovementComponent|SetMaxWalkSpeed (Variables|Character|GetCharacterMovement) (Variables|DesignerVariables|GetPlayerSpeed))
  (Camera|SetFieldOfView (Variables|Default|GetCamera) (Variables|DesignerVariables|GetDefault_FOV)))

(event EventSpaceBarAction
  ;[0.08333 0.08333 0] keyboard inputs
  (Character|Jump))

(event EventScrollWheelAction
  (params (Value :type Float%20%28double-precision%29))
  ;[0 0.0625 0.0625] mouse Inputs
  (CallFunction|CameraZoom Value))

(event EventLeftClickAction
  ;[0 0.0625 0.0625] mouse Inputs
)

(event EventRightClickAction
  ;[0 0.0625 0.0625] mouse Inputs
)

(event EventMouseMovement
  (params (Value :type Vector%202D%20Structure))
  ;[0 0.0625 0.0625] mouse Inputs
  (CallFunction|RotateCamera Value))

(event EventMoveCharacter
  (params (Value :type Vector%202D%20Structure))
  ;[0.08333 0.08333 0] keyboard inputs
  (CallFunction|Moving Value))

(fn WhoPossessesActor
  (bind _asplayer_controller (Utilities|Casting|CastToPlayerController (Pawn|GetController self))
    (:then
      (return true _asplayer_controller 0))
    (:CastFailed
      (return false 0 (AI|GetAIController self)))))