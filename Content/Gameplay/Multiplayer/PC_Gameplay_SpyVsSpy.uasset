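; Player controller for Spy vs Spy multiplayer gameplay that routes player input to the controlled pawn.
; On BeginPlay it adds the gameplay Enhanced Input mapping context.
; Each input action for movement, mouse clicks, scroll wheel, mouse movement and space bar forwards to the pawn as a message call, leaving the actual behavior to the pawn.
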(event EventBeginPlay
  ;[0.08333 0.08333 0] enables player input
  (Input|AddMappingContext (PlayerController|LocalPlayerSubsystems|GetEnhancedInputLocalPlayerSubsystem self) "/Game/Gameplay/Inputs/Gameplay/IMC_Gameplay.IMC_Gameplay" 0 "(bIgnoreAllPressedKeysUntilRelease=True,bForceImmediately=False,bNotifyUserSettings=False)"))

(fn ConstructionScript)

(event Input|EnhancedActionEvents|EnhancedInputActionIA_CharacterMovement
  (params (ActionValue :type Vector%202D%20Structure) (ElapsedSeconds :type Float%20%28double-precision%29) (TriggeredSeconds :type Float%20%28double-precision%29) (InputAction :type Input%20Action%20Object%20Reference :default "/Game/Gameplay/Inputs/Gameplay/IA_CharacterMovement.IA_CharacterMovement"))
  (Class|BPIGameplay|MoveCharacter(Message) (Pawn|GetControlledPawn) ActionValue))

(event Input|EnhancedActionEvents|EnhancedInputActionIA_Mouse_LeftClick
  (params (ActionValue :type Boolean) (ElapsedSeconds :type Float%20%28double-precision%29) (TriggeredSeconds :type Float%20%28double-precision%29) (InputAction :type Input%20Action%20Object%20Reference :default "/Game/Gameplay/Inputs/Gameplay/IA_Mouse_LeftClick.IA_Mouse_LeftClick"))
  (Class|BPIGameplay|LeftClickAction(Message) (Pawn|GetControlledPawn)))

(event Input|EnhancedActionEvents|EnhancedInputActionIA_Mouse_Movement
  (params (ActionValue :type Vector%202D%20Structure) (ElapsedSeconds :type Float%20%28double-precision%29) (TriggeredSeconds :type Float%20%28double-precision%29) (InputAction :type Input%20Action%20Object%20Reference :default "/Game/Gameplay/Inputs/Gameplay/IA_Mouse_Movement.IA_Mouse_Movement"))
  (Class|BPIGameplay|MouseMovement(Message) (Pawn|GetControlledPawn) ActionValue))

(event Input|EnhancedActionEvents|EnhancedInputActionIA_Mouse_RightClick
  (params (ActionValue :type Boolean) (ElapsedSeconds :type Float%20%28double-precision%29) (TriggeredSeconds :type Float%20%28double-precision%29) (InputAction :type Input%20Action%20Object%20Reference :default "/Game/Gameplay/Inputs/Gameplay/IA_Mouse_RightClick.IA_Mouse_RightClick"))
  (Class|BPIGameplay|RightClickAction(Message) (Pawn|GetControlledPawn)))

(event Input|EnhancedActionEvents|EnhancedInputActionIA_Mouse_ScrollWheel
  (params (ActionValue :type Float%20%28double-precision%29) (ElapsedSeconds :type Float%20%28double-precision%29) (TriggeredSeconds :type Float%20%28double-precision%29) (InputAction :type Input%20Action%20Object%20Reference :default "/Game/Gameplay/Inputs/Gameplay/IA_Mouse_ScrollWheel.IA_Mouse_ScrollWheel"))
  (Class|BPIGameplay|ScrollWheelAction(Message) (Pawn|GetControlledPawn) ActionValue))

(event Input|EnhancedActionEvents|EnhancedInputActionIA_SpaceBar
  (params (ActionValue :type Boolean) (ElapsedSeconds :type Float%20%28double-precision%29) (TriggeredSeconds :type Float%20%28double-precision%29) (InputAction :type Input%20Action%20Object%20Reference :default "/Game/Gameplay/Inputs/Gameplay/IA_SpaceBar.IA_SpaceBar"))
  (Class|BPIGameplay|SpaceBarAction(Message) (Pawn|GetControlledPawn)))